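; BP_FlyingAIController is an AI controller in a test folder, named for a flying enemy.
; On possession it runs the BT_AnotherTestEnemy behavior tree and has no other active logic.
; A disconnected chain would seed patrol blackboard keys for patrol mode, direction and current index, but it never executes.
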(event EventBeginPlay)

(event EventTick
  (params (DeltaSeconds :type Float%20%28single-precision%29)))

(event EventPossess
  (params (PossessedPawn :type Pawn%20Object%20Reference))
  (AI|RunBehaviorTree "/Game/ODH/Test/BT_AnotherTestEnemy.BT_AnotherTestEnemy"))

(fn ConstructionScript)
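; Flying enemy test Blueprint that feeds patrol state to its AI through Blackboard keys.
; BeginPlay builds a patrol array from its start location and three patrol components, then seeds the self reference, patrol flag, direction and index.
; ChangeTargetLocation writes the current point and steps the index by IsForward, without bounds checks or direction flips.
; Hearing and sight handling for investigation and combat keys exists but is disconnected and never runs.
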(event EventBeginPlay
  (Variables|Default|SetPatrolArray (Utilities|Array|MakeArray (Transformation|GetActorLocation) (Transformation|GetWorldLocation (Variables|Default|GetPatrolArray1)) (Transformation|GetWorldLocation (Variables|Default|GetPatrolArray2)) (Transformation|GetWorldLocation (Variables|Default|GetPatrolArray3))))
  (AI|Components|Blackboard|SetValueasObject (AI|GetBlackboard 0) (Utilities|Name|MakeLiteralName "MyEnemy") self)
  (AI|Components|Blackboard|SetValueasBool (AI|GetBlackboard 0) (Utilities|Name|MakeLiteralName "IsPatrol") (Variables|Default|GetIsPatrolAI))
  (AI|Components|Blackboard|SetValueasBool (AI|GetBlackboard 0) (Utilities|Name|MakeLiteralName "IsForward") true)
  (Class|BlackboardComponent|SetValueasInt (AI|GetBlackboard 0) (Utilities|Name|MakeLiteralName "CurPatrolIndex")))

(event Collision|EventActorBeginOverlap
  (params (OtherActor :type Actor%20Object%20Reference)))

(event EventTick
  (params (DeltaSeconds :type Float%20%28single-precision%29)))

(fn ConstructionScript)

(fn ChangeTargetLocation
  (bind _returnvalue (Utilities|Name|MakeLiteralName "CurPatrolIndex"))
  (bind _returnvalue_2 (AI|GetBlackboard 0))
  (bind _returnvalue_3 (Utilities|Name|MakeLiteralName "CurPatrolIndex"))
  (bind _returnvalue_4 (AI|GetBlackboard 0))
  (bind _returnvalue_5 (Class|BlackboardComponent|GetValueasInt _returnvalue_2 _returnvalue_3))
  (bind _returnvalue_6 (Class|BlackboardComponent|GetValueasInt _returnvalue_4 _returnvalue))
  (if (ScalableFloat|GetValueasBool (AI|GetBlackboard 0) (Utilities|Name|MakeLiteralName "IsForward"))
    (AI|Components|Blackboard|SetValueasVector _returnvalue_2 (Utilities|Name|MakeLiteralName "PatrolPoint") (Utilities|Array|Get(acopy) (Variables|Default|GetPatrolArray) _returnvalue_5))
    (Class|BlackboardComponent|SetValueasInt (AI|GetBlackboard 0) (Utilities|Name|MakeLiteralName "CurPatrolIndex") (+ _returnvalue_5 1))
    (else
      (AI|Components|Blackboard|SetValueasVector _returnvalue_4 (Utilities|Name|MakeLiteralName "PatrolPoint") (Utilities|Array|Get(acopy) (Variables|Default|GetPatrolArray) _returnvalue_6))
      (Class|BlackboardComponent|SetValueasInt (AI|GetBlackboard 0) (Utilities|Name|MakeLiteralName "CurPatrolIndex") (- _returnvalue_6 1)))))
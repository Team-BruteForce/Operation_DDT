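; AI controller for the skeleton enemy that starts its behavior tree when play begins.
; On BeginPlay it runs BT_SkeletonEnemy, then seeds the blackboard with the IsPatrol flag from its IsPatrolAI variable and an initial forward direction and patrol index.
; It has no active Tick or construction logic.
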(event EventBeginPlay
  (AI|RunBehaviorTree "/Game/ODH/SkeletonEnemy/BT_SkeletonEnemy.BT_SkeletonEnemy")
  (AI|Components|Blackboard|SetValueasBool (AI|GetBlackboard 0) (Utilities|Name|MakeLiteralName "IsPatrol") (Variables|Default|GetIsPatrolAI))
  (AI|Components|Blackboard|SetValueasBool (AI|GetBlackboard 0) (Utilities|Name|MakeLiteralName "IsForward") true)
  (Class|BlackboardComponent|SetValueasInt (AI|GetBlackboard 0) (Utilities|Name|MakeLiteralName "CurPatrolIndex")))

(event EventTick
  (params (DeltaSeconds :type Float%20%28single-precision%29)))

(fn ConstructionScript)
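; Flower enemy Blueprint that seeds its AI Blackboard for patrolling and combo, dash and ranged attacks.
; On BeginPlay it builds a four-point patrol array from its spawn location and three marker components' world locations.
; It then writes a self reference, patrol state, attack-complete flags, a randomized dash attack time limit and a starting ranged attack gauge to the Blackboard.
; The Blueprint itself holds no movement or attack logic.
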(event EventBeginPlay
  (Variables|Default|SetPatrolArray (Utilities|Array|MakeArray (Transformation|GetActorLocation) (Transformation|GetWorldLocation (Variables|Default|GetPatrolArray1)) (Transformation|GetWorldLocation (Variables|Default|GetPatrolArray2)) (Transformation|GetWorldLocation (Variables|Default|GetPatrolArray3))))
  (AI|Components|Blackboard|SetValueasObject (AI|GetBlackboard 0) (Utilities|Name|MakeLiteralName "MyEnemy") self)
  (AI|Components|Blackboard|SetValueasBool (AI|GetBlackboard 0) (Utilities|Name|MakeLiteralName "IsPatrol") (Variables|Default|GetIsPatrolAI))
  (AI|Components|Blackboard|SetValueasBool (AI|GetBlackboard 0) (Utilities|Name|MakeLiteralName "IsForward") true)
  (Class|BlackboardComponent|SetValueasInt (AI|GetBlackboard 0) (Utilities|Name|MakeLiteralName "CurPatrolIndex"))
  (AI|Components|Blackboard|SetValueasFloat (AI|GetBlackboard 0) (Utilities|Name|MakeLiteralName "DashAttackLimiteTime") (Math|Random|RandomFloatinRange 3.0 4.0))
  (AI|Components|Blackboard|SetValueasBool (AI|GetBlackboard 0) (Utilities|Name|MakeLiteralName "IsComboAttackComplete") true)
  (AI|Components|Blackboard|SetValueasBool (AI|GetBlackboard 0) (Utilities|Name|MakeLiteralName "IsDashAttackComplete") true)
  (AI|Components|Blackboard|SetValueasBool (AI|GetBlackboard 0) (Utilities|Name|MakeLiteralName "IsRangedAttackComplete") true)
  (Class|BlackboardComponent|SetValueasInt (AI|GetBlackboard 0) (Utilities|Name|MakeLiteralName "IsRangedAttackGage") 100))

(event Collision|EventActorBeginOverlap
  (params (OtherActor :type Actor%20Object%20Reference)))

(event EventTick
  (params (DeltaSeconds :type Float%20%28single-precision%29)))

(fn ConstructionScript)
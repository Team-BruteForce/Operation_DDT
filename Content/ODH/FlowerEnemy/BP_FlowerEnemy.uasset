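; Flower enemy Blueprint that prepares patrol points and blackboard state for its AI, including combo, dash and ranged attack flags.
; BeginPlay builds PatrolArray from its start location and three patrol components, then sets initial keys, with a randomized dash attack timer.
; AllReset restores the same keys except IsPlayerInBoss, which only the first reset sets.
; StartAbsorbAnimation has AbsorbActor play a dissolve on the mesh.
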(event EventBeginPlay
  (Variables|Default|SetPatrolArray (Utilities|Array|MakeArray (Transformation|GetActorLocation) (Transformation|GetWorldLocation (Variables|Default|GetPatrolArray1)) (Transformation|GetWorldLocation (Variables|Default|GetPatrolArray2)) (Transformation|GetWorldLocation (Variables|Default|GetPatrolArray3))))
  (CallFunction|FirstBlackBoardReset))

(event Collision|EventActorBeginOverlap
  (params (OtherActor :type Actor%20Object%20Reference)))

(event EventTick
  (params (DeltaSeconds :type Float%20%28single-precision%29)))

(event EventAllReset
  (CallFunction|BlackBoardReset))

(event EventStartAbsorbAnimation
  (Default|PlayDissolve (Variables|AbsorbActor|GetAbsorbActor) (Variables|Character|GetMesh)))

(fn ConstructionScript)

(fn FirstBlackBoardReset
  (AI|Components|Blackboard|SetValueasBool (AI|GetBlackboard 0) (Utilities|Name|MakeLiteralName "IsPatrol") (Variables|Default|GetIsPatrolAI))
  (AI|Components|Blackboard|SetValueasBool (AI|GetBlackboard 0) (Utilities|Name|MakeLiteralName "IsForward") true)
  (Class|BlackboardComponent|SetValueasInt (AI|GetBlackboard 0) (Utilities|Name|MakeLiteralName "CurPatrolIndex"))
  (AI|Components|Blackboard|SetValueasFloat (AI|GetBlackboard 0) (Utilities|Name|MakeLiteralName "DashAttackLimiteTime") (Math|Random|RandomFloatinRange 7.0 8.0))
  (AI|Components|Blackboard|SetValueasBool (AI|GetBlackboard 0) (Utilities|Name|MakeLiteralName "IsComboAttack") false)
  (AI|Components|Blackboard|SetValueasBool (AI|GetBlackboard 0) (Utilities|Name|MakeLiteralName "IsDashAttack") false)
  (AI|Components|Blackboard|SetValueasBool (AI|GetBlackboard 0) (Utilities|Name|MakeLiteralName "IsComboAttackComplete") true)
  (AI|Components|Blackboard|SetValueasBool (AI|GetBlackboard 0) (Utilities|Name|MakeLiteralName "IsDashAttackComplete") true)
  (AI|Components|Blackboard|SetValueasBool (AI|GetBlackboard 0) (Utilities|Name|MakeLiteralName "IsInvestigating") false)
  (AI|Components|Blackboard|SetValueasBool (AI|GetBlackboard 0) (Utilities|Name|MakeLiteralName "IsRangedAttack") false)
  (AI|Components|Blackboard|SetValueasBool (AI|GetBlackboard 0) (Utilities|Name|MakeLiteralName "IsRangedAttackComplete") true)
  (Class|BlackboardComponent|SetValueasInt (AI|GetBlackboard 0) (Utilities|Name|MakeLiteralName "IsRangedAttackGage"))
  (AI|Components|Blackboard|SetValueasBool (AI|GetBlackboard 0) (Utilities|Name|MakeLiteralName "IsPlayerInBoss") false))

(fn BlackBoardReset
  (AI|Components|Blackboard|SetValueasBool (AI|GetBlackboard 0) (Utilities|Name|MakeLiteralName "IsPatrol") (Variables|Default|GetIsPatrolAI))
  (AI|Components|Blackboard|SetValueasBool (AI|GetBlackboard 0) (Utilities|Name|MakeLiteralName "IsForward") true)
  (Class|BlackboardComponent|SetValueasInt (AI|GetBlackboard 0) (Utilities|Name|MakeLiteralName "CurPatrolIndex"))
  (AI|Components|Blackboard|SetValueasFloat (AI|GetBlackboard 0) (Utilities|Name|MakeLiteralName "DashAttackLimiteTime") (Math|Random|RandomFloatinRange 7.0 8.0))
  (AI|Components|Blackboard|SetValueasBool (AI|GetBlackboard 0) (Utilities|Name|MakeLiteralName "IsComboAttack") false)
  (AI|Components|Blackboard|SetValueasBool (AI|GetBlackboard 0) (Utilities|Name|MakeLiteralName "IsDashAttack") false)
  (AI|Components|Blackboard|SetValueasBool (AI|GetBlackboard 0) (Utilities|Name|MakeLiteralName "IsComboAttackComplete") true)
  (AI|Components|Blackboard|SetValueasBool (AI|GetBlackboard 0) (Utilities|Name|MakeLiteralName "IsDashAttackComplete") true)
  (AI|Components|Blackboard|SetValueasBool (AI|GetBlackboard 0) (Utilities|Name|MakeLiteralName "IsInvestigating") false)
  (AI|Components|Blackboard|SetValueasBool (AI|GetBlackboard 0) (Utilities|Name|MakeLiteralName "IsRangedAttack") false)
  (AI|Components|Blackboard|SetValueasBool (AI|GetBlackboard 0) (Utilities|Name|MakeLiteralName "IsRangedAttackComplete") true)
  (Class|BlackboardComponent|SetValueasInt (AI|GetBlackboard 0) (Utilities|Name|MakeLiteralName "IsRangedAttackGage")))
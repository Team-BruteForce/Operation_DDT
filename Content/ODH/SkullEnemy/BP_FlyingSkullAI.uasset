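; BP_FlyingSkullAI is the AI logic for the flying skull enemy, which is driven by the BT_SkullEnemy behavior tree.
; On BeginPlay it runs the tree, then seeds the blackboard with the IsPatrolAI flag and starting patrol state: forward direction and first index.
; The Blueprint does no per-tick work, so all further behavior is left to the tree.
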(event EventBeginPlay
  (AI|RunBehaviorTree "/Game/ODH/SkullEnemy/BT_SkullEnemy.BT_SkullEnemy")
  (AI|Components|Blackboard|SetValueasBool (AI|GetBlackboard 0) (Utilities|Name|MakeLiteralName "IsPatrol") (Variables|Default|GetIsPatrolAI))
  (AI|Components|Blackboard|SetValueasBool (AI|GetBlackboard 0) (Utilities|Name|MakeLiteralName "IsForward") true)
  (Class|BlackboardComponent|SetValueasInt (AI|GetBlackboard 0) (Utilities|Name|MakeLiteralName "CurPatrolIndex")))

(event EventTick
  (params (DeltaSeconds :type Float%20%28single-precision%29)))

(fn ConstructionScript)
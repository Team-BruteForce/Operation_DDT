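; BP_Absorb_SK_3 is an example absorb VFX Blueprint for a child skeletal mesh of BP_Boss, but its effect chain is disconnected and BeginPlay is empty.
; That chain hides the mesh, swaps materials and attaches NS_Absorb_SK_3, passing spawn rate and a Feather6_R socket location from the construction script.
; A reversed timeline drives Mask_3 in MPC_Mask, then reveals the mesh with a second material set.
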(event EventBeginPlay)

(fn ConstructionScript
  (Variables|Default|SetLocation (Transformation|GetSocketLocation (Variables|Default|GetAs%20Skeletal%20Mesh%20Component) "Feather6_R")))
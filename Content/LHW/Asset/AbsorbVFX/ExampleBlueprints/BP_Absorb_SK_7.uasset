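; Absorb VFX controller that plays a material dissolve on BP_Boss, its first child mesh (wings) and BP_HolySword, with a separate death variant.
; Each trigger finds actors by class, swaps materials and attaches Niagara systems fed SpawnRate and, for wings and sword, a Location below the boss.
; Timelines animate MPC_Mask scalars, with wings and sword sharing Mask_3 and the body using Mask_7.
; The non-death trigger also calls BP_NormalSword and swaps materials again when reversed timelines finish.
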(event EventTriggerDissolveEffect
  (bind _returnvalue (Actor|GetActorOfClass "/Game/LHW/Blueprint/BP_NormalSword.BP_NormalSword_C"))
  (Default|NewFunction _returnvalue)
  (Utilities|FlowControl|Sequence
    (:then_0
      (bind _returnvalue_2 (Actor|GetActorOfClass "/Game/LHW/Blueprint/BP_Boss.BP_Boss_C"))
      (bind _asskeletal_mesh_component (Utilities|Casting|CastToSkeletalMeshComponent (Components|GetChildComponent (Variables|/Script/Engine.Character|GetMesh _returnvalue_2) 0)))
      (bind _output_get (Variables|Default|SetAs%20Skeletal%20Mesh%20Component _asskeletal_mesh_component))
      (Rendering|SetVisibility _output_get false false)
      (for _index (range 0 (- (Rendering|Material|GetNumMaterials (Variables|Default|GetAs%20Skeletal%20Mesh%20Component)) 1))
        (Rendering|Material|SetMaterial (Variables|Default|GetAs%20Skeletal%20Mesh%20Component) _index (Utilities|Array|Get(acopy) (Variables|Default|GetMaterial%20wing) _index)))
      (bind _returnvalue_3 (Niagara|SpawnSystemAttached "/Game/LHW/Asset2/AbsorbVFX/Niagara/NS_Absorb_SK_3.NS_Absorb_SK_3" (Variables|Default|GetAs%20Skeletal%20Mesh%20Component) "None" "0, 0, 0" "0, 0, 0" "KeepRelativeOffset" false))
      (Niagara|SetNiagaraVariable(Vector3) _returnvalue_3 "Location" (Variables|Default|GetLocation))
      (Niagara|SetNiagaraVariable(Float) _returnvalue_3 "SpawnRate" (Variables|Default|GetSpawnRate))
      (Components|Timeline|SetPlayRate (Variables|Default|GetTimeline_0) 1.0)
      (Utilities|FlowControl|Sequence
        (:then_1
          (bind _newtrack_0 (Timeline|Timeline_1 ReverseFromEnd)
            (:Update
              (Rendering|Material|SetScalarParameterValue "/Game/LHW/Asset2/AbsorbVFX/DemoRoom/SkeletalMeshExample/Character/Materials/Dissolve/New/MPC_Mask.MPC_Mask" "Mask_3" (Math|Float|Lerp -1e+01 1e+01 _newtrack_0) :!class /Script/Engine.KismetMaterialLibrary))
            (:Finished
              (Rendering|SetVisibility (Variables|Default|GetAs%20Skeletal%20Mesh%20Component) true false)
              (for _index_2 (range 0 (- (Rendering|Material|GetNumMaterials (Variables|Default|GetAs%20Skeletal%20Mesh%20Component)) 1))
                (Rendering|Material|SetMaterial (Variables|Default|GetAs%20Skeletal%20Mesh%20Component) _index_2 (Utilities|Array|Get(acopy) (Variables|Default|GetMaterial%20wing2) _index_2))))))))
    (:then_1
      (bind _returnvalue_4 (Actor|GetActorOfClass "/Game/LHW/Blueprint/BP_Boss.BP_Boss_C"))
      (bind _output_get_2 (Variables|Default|SetMesh (Variables|/Script/Engine.Character|GetMesh _returnvalue_4)))
      (Rendering|SetVisibility _output_get_2 true false)
      (for _index_3 (range 0 (- (Rendering|Material|GetNumMaterials (Variables|Default|GetMesh)) 1))
        (Rendering|Material|SetMaterial (Variables|Default|GetMesh) _index_3 (Utilities|Array|Get(acopy) (Variables|Default|GetMaterial_Metal) _index_3)))
      (Utilities|FlowControl|Delay 1.0)
      (bind _returnvalue_5 (Niagara|SpawnSystemAttached "/Game/LHW/Asset/AbsorbVFX/Niagara/NS_Absorb_SK_7.NS_Absorb_SK_7" (Variables|Default|GetMesh) "None" "0, 0, 0" "0, 0, 0" "KeepRelativeOffset" false))
      (Niagara|SetNiagaraVariable(Float) _returnvalue_5 "SpawnRate" (Variables|Default|GetSpawnRate))
      (Components|Timeline|SetPlayRate (Variables|Default|GetTimeline_0) 0.25)
      (Utilities|FlowControl|Sequence
        (:then_1
          (Components|Timeline|SetPlayRate (Variables|Default|GetTimeline_0) 0.2)
          (Utilities|FlowControl|Sequence
            (:then_0
              (bind _newtrack_0_2 (Timeline|Timeline_0 PlayFromStart)
                (:Update
                  (Rendering|Material|SetScalarParameterValue "/Game/LHW/Asset/AbsorbVFX/DemoRoom/SkeletalMeshExample/Character/Materials/Dissolve/New/MPC_Mask.MPC_Mask" "Mask_7" (Math|Float|Lerp -1e+01 1.0 _newtrack_0_2) :!class /Script/Engine.KismetMaterialLibrary))))
            (:then_1
              (for _index_4 (range 2 (- (Rendering|Material|GetNumMaterials (Variables|Default|GetMesh)) 1))
                (Rendering|Material|SetMaterial (Variables|Default|GetMesh) _index_4 (Utilities|Array|Get(acopy) (Variables|Default|GetMaterial_Golden) _index_4))
                (bind _newtrack_0_3 (Timeline|Timeline ReverseFromEnd)
                  (:Update
                    (Rendering|Material|SetScalarParameterValue "/Game/LHW/Asset/AbsorbVFX/DemoRoom/SkeletalMeshExample/Character/Materials/Dissolve/New/MPC_Mask.MPC_Mask" "Mask_7" (Math|Float|Lerp -1e+01 1.0 _newtrack_0_3) :!class /Script/Engine.KismetMaterialLibrary))
                  (:Finished
                    (for _index_5 (range 0 (- (Rendering|Material|GetNumMaterials (Variables|Default|GetMesh)) 1))
                      (Rendering|Material|SetMaterial (Variables|Default|GetMesh) _index_5 (Utilities|Array|Get(acopy) (Variables|Default|GetMaterial) _index_5)))))))))))
    (:then_2
      (bind _returnvalue_6 (Actor|GetActorOfClass "/Game/LHW/Blueprint/BP_HolySword.BP_HolySword_C"))
      (Variables|Default|SetSwordMesh (Variables|/Script/Operration_DDT.CBossWeapon|GetSkeletalMesh _returnvalue_6))
      (Rendering|SetVisibility (Variables|Default|GetSwordMesh) true false)
      (for _index_6 (range 0 (- (Rendering|Material|GetNumMaterials (Variables|Default|GetSwordMesh)) 1))
        (Rendering|Material|SetMaterial (Variables|Default|GetSwordMesh) _index_6 (Utilities|Array|Get(acopy) (Variables|Default|GetSwordMeterial) _index_6)))
      (bind _returnvalue_7 (Niagara|SpawnSystemAttached "/Game/LHW/Asset2/AbsorbVFX/Niagara/NS_Absorb_SK_5.NS_Absorb_SK_5" (Variables|Default|GetSwordMesh) "None" "0, 0, 0" "0, 0, 0" "KeepRelativeOffset" false))
      (Niagara|SetNiagaraVariable(Vector3) _returnvalue_7 "Location" (Variables|Default|GetLocation))
      (Niagara|SetNiagaraVariable(Float) _returnvalue_7 "SpawnRate" (Variables|Default|GetSpawnRate))
      (Components|Timeline|SetPlayRate (Variables|Default|GetTimeline_4) 1.0)
      (Utilities|FlowControl|Sequence
        (:then_1
          (bind _newtrack_0_4 (Timeline|Timeline_4 ReverseFromEnd)
            (:Update
              (Rendering|Material|SetScalarParameterValue "/Game/LHW/Asset2/AbsorbVFX/DemoRoom/SkeletalMeshExample/Character/Materials/Dissolve/New/MPC_Mask.MPC_Mask" "Mask_3" (Math|Float|Lerp -1e+01 1e+01 _newtrack_0_4) :!class /Script/Engine.KismetMaterialLibrary))
            (:Finished
              (Rendering|SetVisibility (Variables|Default|GetSwordMesh) true false)
              (for _index_7 (range 0 (- (Rendering|Material|GetNumMaterials (Variables|Default|GetSwordMesh)) 1))
                (Rendering|Material|SetMaterial (Variables|Default|GetSwordMesh) _index_7 (Utilities|Array|Get(acopy) (Variables|Default|GetSwordMeterial_0) _index_7))))))))))

(event EventTriggerDissolveEffectDead
  (Utilities|FlowControl|Sequence
    (:then_0
      (bind _returnvalue (Actor|GetActorOfClass "/Game/LHW/Blueprint/BP_Boss.BP_Boss_C"))
      (bind _output_get (Variables|Default|SetMesh (Variables|/Script/Engine.Character|GetMesh _returnvalue)))
      (Rendering|SetVisibility _output_get true false)
      (for _index (range 0 (- (Rendering|Material|GetNumMaterials (Variables|Default|GetMesh)) 1))
        (Rendering|Material|SetMaterial (Variables|Default|GetMesh) _index (Utilities|Array|Get(acopy) (Variables|Default|GetMaterial_Golden) _index)))
      (Utilities|FlowControl|Delay 1.0)
      (bind _returnvalue_2 (Niagara|SpawnSystemAttached "/Game/LHW/Asset2/AbsorbVFX/Niagara/NS_Absorb_SK_4.NS_Absorb_SK_4" (Variables|Default|GetMesh) "None" "0, 0, 0" "0, 0, 0" "KeepRelativeOffset" false))
      (Niagara|SetNiagaraVariable(Float) _returnvalue_2 "SpawnRate" (Variables|Default|GetSpawnRate))
      (Components|Timeline|SetPlayRate (Variables|Default|GetTimeline_0) 0.25)
      (Utilities|FlowControl|Sequence
        (:then_1
          (Components|Timeline|SetPlayRate (Variables|Default|GetTimeline_0) 0.2)
          (Utilities|FlowControl|Sequence
            (:then_0
              (bind _newtrack_0 (Timeline|Timeline_2 PlayFromStart)
                (:Update
                  (Rendering|Material|SetScalarParameterValue "/Game/LHW/Asset/AbsorbVFX/DemoRoom/SkeletalMeshExample/Character/Materials/Dissolve/New/MPC_Mask.MPC_Mask" "Mask_7" (Math|Float|Lerp -1e+01 2.0 _newtrack_0) :!class /Script/Engine.KismetMaterialLibrary))))))))
    (:then_1
      (bind _returnvalue_3 (Actor|GetActorOfClass "/Game/LHW/Blueprint/BP_Boss.BP_Boss_C"))
      (bind _asskeletal_mesh_component (Utilities|Casting|CastToSkeletalMeshComponent (Components|GetChildComponent (Variables|/Script/Engine.Character|GetMesh _returnvalue_3) 0)))
      (bind _output_get_2 (Variables|Default|SetAs%20Skeletal%20Mesh%20Component _asskeletal_mesh_component))
      (Rendering|SetVisibility _output_get_2 false false)
      (for _index_2 (range 0 (- (Rendering|Material|GetNumMaterials (Variables|Default|GetAs%20Skeletal%20Mesh%20Component)) 1))
        (Rendering|Material|SetMaterial (Variables|Default|GetAs%20Skeletal%20Mesh%20Component) _index_2 (Utilities|Array|Get(acopy) (Variables|Default|GetMaterial%20wing) _index_2)))
      (bind _returnvalue_4 (Niagara|SpawnSystemAttached "/Game/LHW/Asset2/AbsorbVFX/Niagara/NS_Absorb_SK_4.NS_Absorb_SK_4" (Variables|Default|GetAs%20Skeletal%20Mesh%20Component) "None" "0, 0, 0" "0, 0, 0" "KeepRelativeOffset" false))
      (Niagara|SetNiagaraVariable(Vector3) _returnvalue_4 "Location" (Variables|Default|GetLocation))
      (Niagara|SetNiagaraVariable(Float) _returnvalue_4 "SpawnRate" (Variables|Default|GetSpawnRate))
      (Components|Timeline|SetPlayRate (Variables|Default|GetTimeline_0) 1.0)
      (Utilities|FlowControl|Sequence
        (:then_1
          (bind _newtrack_0_2 (Timeline|Timeline_3 PlayFromStart)
            (:Update
              (Rendering|Material|SetScalarParameterValue "/Game/LHW/Asset2/AbsorbVFX/DemoRoom/SkeletalMeshExample/Character/Materials/Dissolve/New/MPC_Mask.MPC_Mask" "Mask_3" (Math|Float|Lerp -1e+01 1e+01 _newtrack_0_2) :!class /Script/Engine.KismetMaterialLibrary))))))
    (:then_2
      (bind _returnvalue_5 (Actor|GetActorOfClass "/Game/LHW/Blueprint/BP_HolySword.BP_HolySword_C"))
      (Variables|Default|SetSwordMesh (Variables|/Script/Operration_DDT.CBossWeapon|GetSkeletalMesh _returnvalue_5))
      (Rendering|SetVisibility (Variables|Default|GetSwordMesh) false false)
      (for _index_3 (range 0 (- (Rendering|Material|GetNumMaterials (Variables|Default|GetSwordMesh)) 1))
        (Rendering|Material|SetMaterial (Variables|Default|GetSwordMesh) _index_3 (Utilities|Array|Get(acopy) (Variables|Default|GetSwordMeterial) _index_3)))
      (bind _returnvalue_6 (Niagara|SpawnSystemAttached "/Game/LHW/Asset2/AbsorbVFX/Niagara/NS_Absorb_SK_4.NS_Absorb_SK_4" (Variables|Default|GetSwordMesh) "None" "0, 0, 0" "0, 0, 0" "KeepRelativeOffset" false))
      (Niagara|SetNiagaraVariable(Vector3) _returnvalue_6 "Location" (Variables|Default|GetLocation))
      (Niagara|SetNiagaraVariable(Float) _returnvalue_6 "SpawnRate" (Variables|Default|GetSpawnRate))
      (Components|Timeline|SetPlayRate (Variables|Default|GetTimeline_4) 1.0)
      (Utilities|FlowControl|Sequence
        (:then_1
          (bind _newtrack_0_3 (Timeline|Timeline_5 PlayFromStart)
            (:Update
              (Rendering|Material|SetScalarParameterValue "/Game/LHW/Asset2/AbsorbVFX/DemoRoom/SkeletalMeshExample/Character/Materials/Dissolve/New/MPC_Mask.MPC_Mask" "Mask_3" (Math|Float|Lerp -1e+01 1e+01 _newtrack_0_3) :!class /Script/Engine.KismetMaterialLibrary))))))))

(fn ConstructionScript
  (bind _returnvalue (Actor|GetActorOfClass "/Game/LHW/Blueprint/BP_Boss.BP_Boss_C"))
  (Variables|Default|SetLocation (- (Transformation|GetActorLocation _returnvalue) "0.000000,0.000000,1000.000000")))